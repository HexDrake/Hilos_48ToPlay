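; Crusher obstacle that moves two cubes and costs a SideScrollerCharacter a life on contact.
; Two looping timers started at BeginPlay fire one event per cube on the same interval.
; Each event drives its cube's relative Y with a timeline, whose Update starts a second timeline on that axis after a delay.
; Two box overlaps cast to the character and call PerderVida.
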(event OnComponentBeginOverlap(Box)
  (params (OverlappedComponent :type Primitive%20Component%20Object%20Reference) (OtherActor :type Actor%20Object%20Reference) (OtherComp :type Primitive%20Component%20Object%20Reference) (OtherBodyIndex :type Integer) (bFromSweep :type Boolean) (SweepResult :type Hit%20Result%20Structure%20%28by%20ref%29))
  (bind _asside_scroller_character (Utilities|Casting|CastToSideScrollerCharacter OtherActor))
  (Default|PerderVida _asside_scroller_character 1.0)
  (Utilities|FlowControl|Delay 1.0))

(event OnComponentBeginOverlap(Box1)
  (params (OverlappedComponent :type Primitive%20Component%20Object%20Reference) (OtherActor :type Actor%20Object%20Reference) (OtherComp :type Primitive%20Component%20Object%20Reference) (OtherBodyIndex :type Integer) (bFromSweep :type Boolean) (SweepResult :type Hit%20Result%20Structure%20%28by%20ref%29))
  (bind _asside_scroller_character (Utilities|Casting|CastToSideScrollerCharacter OtherActor))
  (Default|PerderVida _asside_scroller_character 1.0)
  (Utilities|FlowControl|Delay 1.0))

(event Custom|Aplastar_der
  (bind _newtrack_0 (Timeline|Timeline_2 PlayFromStart)
    (:Update
      (Transformation|SetRelativeLocation (Variables|Default|GetCube2) (Math|Vector|MakeVector 0.0 _newtrack_0 0.0) false false)
      (Utilities|FlowControl|Delay 2.0)
      (bind _newtrack_0_2 (Timeline|Timeline_3 PlayFromStart)
        (:Update
          (Transformation|SetRelativeLocation (Variables|Default|GetCube2) (Math|Vector|MakeVector 0.0 _newtrack_0_2 0.0) false false)
          (Utilities|FlowControl|Delay 1.0))))))

(event Custom|Aplastar
  (bind _newtrack_0 (Timeline|Timeline_0 PlayFromStart)
    (:Update
      (Transformation|SetRelativeLocation (Variables|Default|GetCube) (Math|Vector|MakeVector 0.0 _newtrack_0 0.0) false false)
      (Utilities|FlowControl|Delay 2.0)
      (bind _newtrack_0_2 (Timeline|Timeline_1 PlayFromStart)
        (:Update
          (Transformation|SetRelativeLocation (Variables|Default|GetCube) (Math|Vector|MakeVector 0.0 _newtrack_0_2 0.0) false false)
          (Utilities|FlowControl|Delay 1.0))))))

(event EventBeginPlay
  (Utilities|FlowControl|Sequence
    (:then_0
      (Utilities|Time|SetTimerbyFunctionName 0 "Aplastar" 4.0 true))
    (:then_1
      (Utilities|Time|SetTimerbyFunctionName 0 "Aplastar_der" 4.0 true))))

(fn ConstructionScript)