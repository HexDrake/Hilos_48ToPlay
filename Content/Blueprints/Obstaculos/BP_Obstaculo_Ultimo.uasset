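; BP_Obstaculo_Ultimo is an obstacle actor whose cube moves continuously from the moment play begins.
; Two events, Ciclo1 and Ciclo2, each play their own timeline from the start, setting the cube's relative location from a track on every update without sweep.
; Each waits briefly when its timeline finishes, then triggers the other, forming an endless alternating loop.
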(event Custom|Ciclo1
  (bind _newtrack_1 (Timeline|Timeline_0 PlayFromStart)
    (:Update
      (Transformation|SetRelativeLocation (Variables|Default|GetCube) _newtrack_1 false false))
    (:Finished
      (Utilities|FlowControl|Delay 0.2)
      (CallFunction|Ciclo2))))

(event Custom|ciclo2
  (bind _newtrack_1 (Timeline|Timeline_1 PlayFromStart)
    (:Update
      (Transformation|SetRelativeLocation (Variables|Default|GetCube) _newtrack_1 false false))
    (:Finished
      (Utilities|FlowControl|Delay 0.2)
      (CallFunction|Ciclo1))))

(event EventBeginPlay
  (CallFunction|Ciclo1))

(fn ConstructionScript)