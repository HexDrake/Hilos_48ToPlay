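; Dynamic spike trap obstacle for the side-scroller, triggered once when the player character overlaps its box, which then disables overlap events.
; Seven cones move along relative Z on chained timelines: the first starts the second on finish, while later ones restart the next on every update, holding it until the previous stops.
; Each cone hit waits one second, then calls PerderVida on the character to remove half a life point.
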(event OnComponentBeginOverlap(Box)
  (params (OverlappedComponent :type Primitive%20Component%20Object%20Reference) (OtherActor :type Actor%20Object%20Reference) (OtherComp :type Primitive%20Component%20Object%20Reference) (OtherBodyIndex :type Integer) (bFromSweep :type Boolean) (SweepResult :type Hit%20Result%20Structure%20%28by%20ref%29))
  (Utilities|Casting|CastToSideScrollerCharacter OtherActor)
  (CallFunction|Pico01))

(event OnComponentHit(Cone)
  (params (HitComponent :type Primitive%20Component%20Object%20Reference) (OtherActor :type Actor%20Object%20Reference) (OtherComp :type Primitive%20Component%20Object%20Reference) (NormalImpulse :type Vector :default "0, 0, 0") (Hit :type Hit%20Result%20Structure%20%28by%20ref%29))
  (Utilities|FlowControl|Delay 1.0)
  (bind _asside_scroller_character (Utilities|Casting|CastToSideScrollerCharacter OtherActor))
  (Default|PerderVida _asside_scroller_character 0.5))

(event OnComponentHit(Cone1)
  (params (HitComponent :type Primitive%20Component%20Object%20Reference) (OtherActor :type Actor%20Object%20Reference) (OtherComp :type Primitive%20Component%20Object%20Reference) (NormalImpulse :type Vector :default "0, 0, 0") (Hit :type Hit%20Result%20Structure%20%28by%20ref%29))
  (Utilities|FlowControl|Delay 1.0)
  (bind _asside_scroller_character (Utilities|Casting|CastToSideScrollerCharacter OtherActor))
  (Default|PerderVida _asside_scroller_character 0.5))

(event OnComponentHit(Cone2)
  (params (HitComponent :type Primitive%20Component%20Object%20Reference) (OtherActor :type Actor%20Object%20Reference) (OtherComp :type Primitive%20Component%20Object%20Reference) (NormalImpulse :type Vector :default "0, 0, 0") (Hit :type Hit%20Result%20Structure%20%28by%20ref%29))
  (Utilities|FlowControl|Delay 1.0)
  (bind _asside_scroller_character (Utilities|Casting|CastToSideScrollerCharacter OtherActor))
  (Default|PerderVida _asside_scroller_character 0.5))

(event OnComponentHit(Cone3)
  (params (HitComponent :type Primitive%20Component%20Object%20Reference) (OtherActor :type Actor%20Object%20Reference) (OtherComp :type Primitive%20Component%20Object%20Reference) (NormalImpulse :type Vector :default "0, 0, 0") (Hit :type Hit%20Result%20Structure%20%28by%20ref%29))
  (Utilities|FlowControl|Delay 1.0)
  (bind _asside_scroller_character (Utilities|Casting|CastToSideScrollerCharacter OtherActor))
  (Default|PerderVida _asside_scroller_character 0.5))

(event OnComponentHit(Cone4)
  (params (HitComponent :type Primitive%20Component%20Object%20Reference) (OtherActor :type Actor%20Object%20Reference) (OtherComp :type Primitive%20Component%20Object%20Reference) (NormalImpulse :type Vector :default "0, 0, 0") (Hit :type Hit%20Result%20Structure%20%28by%20ref%29))
  (Utilities|FlowControl|Delay 1.0)
  (bind _asside_scroller_character (Utilities|Casting|CastToSideScrollerCharacter OtherActor))
  (Default|PerderVida _asside_scroller_character 0.5))

(event OnComponentHit(Cone5)
  (params (HitComponent :type Primitive%20Component%20Object%20Reference) (OtherActor :type Actor%20Object%20Reference) (OtherComp :type Primitive%20Component%20Object%20Reference) (NormalImpulse :type Vector :default "0, 0, 0") (Hit :type Hit%20Result%20Structure%20%28by%20ref%29))
  (Utilities|FlowControl|Delay 1.0)
  (bind _asside_scroller_character (Utilities|Casting|CastToSideScrollerCharacter OtherActor))
  (Default|PerderVida _asside_scroller_character 0.5))

(event OnComponentHit(Cone6)
  (params (HitComponent :type Primitive%20Component%20Object%20Reference) (OtherActor :type Actor%20Object%20Reference) (OtherComp :type Primitive%20Component%20Object%20Reference) (NormalImpulse :type Vector :default "0, 0, 0") (Hit :type Hit%20Result%20Structure%20%28by%20ref%29))
  (Utilities|FlowControl|Delay 1.0)
  (bind _asside_scroller_character (Utilities|Casting|CastToSideScrollerCharacter OtherActor))
  (Default|PerderVida _asside_scroller_character 0.5))

(event Custom|Pico01
  (bind _cone (Variables|Default|GetCone))
  (bind _relativelocation (Variables|/Script/Engine.SceneComponent|GetRelativeLocation _cone))
  (Variables|/Script/Engine.PrimitiveComponent|SetbGenerateOverlapEvents (Variables|Default|GetBox) false)
  (bind _newtrack_0 (Timeline|Timeline_0 PlayFromStart)
    (:Update
      (Transformation|SetRelativeLocation _cone (Math|Vector|MakeVector (.x _relativelocation) (.y _relativelocation) _newtrack_0) false false))
    (:Finished
      (CallFunction|Pico02))))

(event Custom|Pico02
  (bind _cone1 (Variables|Default|GetCone1))
  (bind _relativelocation (Variables|/Script/Engine.SceneComponent|GetRelativeLocation _cone1))
  (bind _newtrack_0 (Timeline|Timeline_1 PlayFromStart)
    (:Update
      (Transformation|SetRelativeLocation _cone1 (Math|Vector|MakeVector (.x _relativelocation) (.y _relativelocation) _newtrack_0) false false)
      (CallFunction|Pico03))))

(event Custom|Pico03
  (bind _cone2 (Variables|Default|GetCone2))
  (bind _relativelocation (Variables|/Script/Engine.SceneComponent|GetRelativeLocation _cone2))
  (bind _newtrack_0 (Timeline|Timeline_2 PlayFromStart)
    (:Update
      (Transformation|SetRelativeLocation _cone2 (Math|Vector|MakeVector (.x _relativelocation) (.y _relativelocation) _newtrack_0) false false)
      (CallFunction|Pico04))))

(event Custom|Pico05
  (bind _cone4 (Variables|Default|GetCone4))
  (bind _relativelocation (Variables|/Script/Engine.SceneComponent|GetRelativeLocation _cone4))
  (bind _newtrack_0 (Timeline|Timeline_4 PlayFromStart)
    (:Update
      (Transformation|SetRelativeLocation _cone4 (Math|Vector|MakeVector (.x _relativelocation) (.y _relativelocation) _newtrack_0) false false)
      (CallFunction|Pico06))))

(event Custom|Pico04
  (bind _cone3 (Variables|Default|GetCone3))
  (bind _relativelocation (Variables|/Script/Engine.SceneComponent|GetRelativeLocation _cone3))
  (bind _newtrack_0 (Timeline|Timeline_3 PlayFromStart)
    (:Update
      (Transformation|SetRelativeLocation _cone3 (Math|Vector|MakeVector (.x _relativelocation) (.y _relativelocation) _newtrack_0) false false)
      (CallFunction|Pico05))))

(event Custom|Pico07
  (bind _cone6 (Variables|Default|GetCone6))
  (bind _relativelocation (Variables|/Script/Engine.SceneComponent|GetRelativeLocation _cone6))
  (bind _newtrack_0 (Timeline|Timeline_6 PlayFromStart)
    (:Update
      (Transformation|SetRelativeLocation _cone6 (Math|Vector|MakeVector (.x _relativelocation) (.y _relativelocation) _newtrack_0) false false))))

(event Custom|Pico06
  (bind _cone5 (Variables|Default|GetCone5))
  (bind _relativelocation (Variables|/Script/Engine.SceneComponent|GetRelativeLocation _cone5))
  (bind _newtrack_0 (Timeline|Timeline_5 PlayFromStart)
    (:Update
      (Transformation|SetRelativeLocation _cone5 (Math|Vector|MakeVector (.x _relativelocation) (.y _relativelocation) _newtrack_0) false false)
      (CallFunction|Pico07))))

(event EventBeginPlay)

(event Collision|EventActorBeginOverlap
  (params (OtherActor :type Actor%20Object%20Reference)))

(event EventTick
  (params (DeltaSeconds :type Float%20%28single-precision%29)))

(fn ConstructionScript)