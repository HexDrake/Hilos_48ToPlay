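; BP_plataforma is an obstacle platform whose Cube moves on a repeating cycle in relative Y and Z.
; BeginPlay starts the piso event immediately and repeats it on a looping four-second timer.
; Piso plays two timelines in sequence, each driving both axes from one track, with the second negating Z to change the diagonal.
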(event Custom|piso
  (bind _newtrack_0 (Timeline|Timeline_0 PlayFromStart)
    (:Update
      (Transformation|SetRelativeLocation (Variables|Default|GetCube) (Math|Vector|MakeVector 0.0 _newtrack_0 _newtrack_0) false false))
    (:Finished
      (bind _newtrack_0_2 (Timeline|Timeline_1 PlayFromStart)
        (:Update
          (Transformation|SetRelativeLocation (Variables|Default|GetCube) (Math|Vector|MakeVector 0.0 _newtrack_0_2 (* _newtrack_0_2 -1.0)) false false))))))

(event EventBeginPlay
  (Utilities|FlowControl|Sequence
    (:then_0
      (Utilities|Time|SetTimerbyFunctionName 0 "piso" 4.0 true))
    (:then_1
      (CallFunction|Piso))))

(fn ConstructionScript)