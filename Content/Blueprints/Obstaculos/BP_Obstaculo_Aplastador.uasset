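; Crusher obstacle for a side scroller that endlessly cycles a Cube through shake, fall and return phases.
; After a configurable start Delay, chained Timelines drive the Cube's relative X and Z, with short pauses between phases.
; The Temblar and Regreso custom events restart each half of the cycle to form the loop.
; Any SideScrollerCharacter that begins overlapping the Box loses life through PerderVida.
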(event OnComponentBeginOverlap(Box)
  (params (OverlappedComponent :type Primitive%20Component%20Object%20Reference) (OtherActor :type Actor%20Object%20Reference) (OtherComp :type Primitive%20Component%20Object%20Reference) (OtherBodyIndex :type Integer) (bFromSweep :type Boolean) (SweepResult :type Hit%20Result%20Structure%20%28by%20ref%29))
  (bind _asside_scroller_character (Utilities|Casting|CastToSideScrollerCharacter OtherActor))
  (Default|PerderVida _asside_scroller_character 1.0))

(event Custom|Temblar
  (bind _cube (Variables|Default|GetCube))
  (bind _newtrack_0 (Timeline|TemblarTime PlayFromStart)
    (:Update
      (Transformation|SetRelativeLocation _cube (Math|Vector|MakeVector _newtrack_0 0.0 3.1e+02) false false))
    (:Finished
      (Utilities|FlowControl|Delay 0.2)
      (bind _newtrack_0_2 (Timeline|Caer PlayFromStart)
        (:Update
          (Transformation|SetRelativeLocation _cube (Math|Vector|MakeVector _newtrack_0 0.0 _newtrack_0_2) false false))
        (:Finished
          (Utilities|FlowControl|Delay 1.0)
          (CallFunction|Regreso))))))

(event Custom|Regreso
  (bind _cube (Variables|Default|GetCube))
  (bind _newtrack_0 (Timeline|Timeline_0 PlayFromStart)
    (:Update
      (Transformation|SetRelativeLocation _cube (Math|Vector|MakeVector _newtrack_0 0.0 0.0) false false))
    (:Finished
      (Utilities|FlowControl|Delay 0.2)
      (bind _newtrack_0_2 (Timeline|Timeline_1 PlayFromStart)
        (:Update
          (Transformation|SetRelativeLocation _cube (Math|Vector|MakeVector _newtrack_0 0.0 _newtrack_0_2) false false))
        (:Finished
          (Utilities|FlowControl|Delay 1.0)
          (CallFunction|Temblar))))))

(event EventBeginPlay
  (bind _cube (Variables|Default|GetCube))
  (Utilities|FlowControl|Delay (Variables|Default|GetDelay))
  (bind _newtrack_0 (Timeline|TemblarTime Play)
    (:Update
      (Transformation|SetRelativeLocation _cube (Math|Vector|MakeVector _newtrack_0 0.0 3.1e+02) false false))
    (:Finished
      (Utilities|FlowControl|Delay 0.2)
      (bind _newtrack_0_2 (Timeline|Caer PlayFromStart)
        (:Update
          (Transformation|SetRelativeLocation _cube (Math|Vector|MakeVector _newtrack_0 0.0 _newtrack_0_2) false false))
        (:Finished
          (Utilities|FlowControl|Delay 1.0)
          (CallFunction|Regreso))))))

(fn ConstructionScript)