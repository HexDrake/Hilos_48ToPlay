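; BP_ZEUS is a Zeus actor that runs a timed, scripted cinematic from BeginPlay.
; After a delay it slides one skeletal mesh into place while setting Yelling, then Magia, then Dance on the Zeus_Animation instances of both meshes.
; Alongside the magic and dance phases it triggers movement on the first BP_Cinematic and starts the first BP_Partioles, with all timing driven by hardcoded Delays.
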(event EventBeginPlay
  (Utilities|FlowControl|Delay 3.8)
  (Components|MoveComponentTo (Variables|Default|GetSkeletalMesh) "-754.898865,-29842.550781,-5289.420898" "0,180.000000, 0" false false 5.0 false)
  (Utilities|FlowControl|Sequence
    (:then_0
      (bind _aszeus_animation (Utilities|Casting|CastToZeus_Animation (Components|SkeletalMesh|GetAnimInstance (Variables|Default|GetSkeletalMesh))))
      (Variables|/Game/Blueprints/zeus/Zeus_Animation.Zeus_Animation_C|SetYelling _aszeus_animation true))
    (:then_1
      (bind _aszeus_animation_2 (Utilities|Casting|CastToZeus_Animation (Components|SkeletalMesh|GetAnimInstance (Variables|Default|GetSkeletalMesh1))))
      (Variables|/Game/Blueprints/zeus/Zeus_Animation.Zeus_Animation_C|SetYelling _aszeus_animation_2 true)
      (Utilities|FlowControl|Delay 6.3)
      (Utilities|FlowControl|Sequence
        (:then_0
          (Variables|/Game/Blueprints/zeus/Zeus_Animation.Zeus_Animation_C|SetMagia _aszeus_animation true))
        (:then_1
          (Variables|/Game/Blueprints/zeus/Zeus_Animation.Zeus_Animation_C|SetMagia _aszeus_animation_2 true)
          (bind _outactors (Actor|GetAllActorsOfClass "/Game/Blueprints/BP_Cinematic.BP_Cinematic_C"))
          (Default|Mov+ (Utilities|Array|Get(acopy) _outactors))
          (bind _outactors_2 (Actor|GetAllActorsOfClass "/Game/Blueprints/BP_Partioles.BP_Partioles_C"))
          (Utilities|FlowControl|Delay 1.3)
          (Default|Init (Utilities|Array|Get(acopy) _outactors_2))
          (Utilities|FlowControl|Delay 5.0)
          (Default|Move2 (Utilities|Array|Get(acopy) _outactors))
          (Utilities|FlowControl|Sequence
            (:then_0
              (Variables|/Game/Blueprints/zeus/Zeus_Animation.Zeus_Animation_C|SetDance _aszeus_animation true))
            (:then_1
              (Variables|/Game/Blueprints/zeus/Zeus_Animation.Zeus_Animation_C|SetDance _aszeus_animation_2 true)
              (Transformation|SetRelativeRotation (Variables|Default|GetSkeletalMesh) "0,270.000000, 0" false false))))))))

(fn ConstructionScript)